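; BP_InteractObject is an interactable actor in the inventory system that tells the player character when it is within range.
; On BeginPlay it caches the player's ThirdPersonCharacter.
; When a "Player"-tagged actor overlaps its collision sphere, it enables CanInteract, registers itself on the character and shows the HUD interact prompt.
; Leaving the sphere clears the reference and flag and hides the prompt.
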(event OnComponentBeginOverlap(CollisionSphere)
  (params (OverlappedComponent :type Primitive%20Component%20Object%20Reference) (OtherActor :type Actor%20Object%20Reference) (OtherComp :type Primitive%20Component%20Object%20Reference) (OtherBodyIndex :type Integer) (bFromSweep :type Boolean) (SweepResult :type Hit%20Result%20Structure%20%28by%20ref%29))
  (if (Actor|ActorHasTag OtherActor "Player")
    (Variables|/Game/ThirdPersonBP/Blueprints/ThirdPersonCharacter.ThirdPersonCharacter_C|SetCanInteract? (Variables|Default|GetCharacterRef) true)
    (Variables|/Game/ThirdPersonBP/Blueprints/ThirdPersonCharacter.ThirdPersonCharacter_C|SetBp_InteractObjects (Variables|Default|GetCharacterRef) self)
    (Widget|SetVisibility (Variables|/Game/GameDesign/JeanDavalos/HUDandUI/W_PlayerHud.W_PlayerHud_C|GetOnScreenCanInteract (Variables|/Game/ThirdPersonBP/Blueprints/ThirdPersonCharacter.ThirdPersonCharacter_C|GetCharacterHudRef (Variables|Default|GetCharacterRef))) "Visible")))

(event OnComponentEndOverlap(CollisionSphere)
  (params (OverlappedComponent :type Primitive%20Component%20Object%20Reference) (OtherActor :type Actor%20Object%20Reference) (OtherComp :type Primitive%20Component%20Object%20Reference) (OtherBodyIndex :type Integer))
  (if (Actor|ActorHasTag OtherActor "Player")
    (Variables|/Game/ThirdPersonBP/Blueprints/ThirdPersonCharacter.ThirdPersonCharacter_C|SetCanInteract? (Variables|Default|GetCharacterRef) false)
    (Variables|/Game/ThirdPersonBP/Blueprints/ThirdPersonCharacter.ThirdPersonCharacter_C|SetBp_InteractObjects (Variables|Default|GetCharacterRef) 0)
    (Widget|SetVisibility (Variables|/Game/GameDesign/JeanDavalos/HUDandUI/W_PlayerHud.W_PlayerHud_C|GetOnScreenCanInteract (Variables|/Game/ThirdPersonBP/Blueprints/ThirdPersonCharacter.ThirdPersonCharacter_C|GetCharacterHudRef (Variables|Default|GetCharacterRef))) "Hidden")))

(event EventBeginPlay
  (bind _asthird_person_character (Utilities|Casting|CastToThirdPersonCharacter (Game|GetPlayerCharacter 0)))
  (Variables|Default|SetCharacterRef _asthird_person_character))

(event Collision|EventActorBeginOverlap
  (params (OtherActor :type Actor%20Object%20Reference)))

(event EventTick
  (params (DeltaSeconds :type Float%20%28single-precision%29)))

(fn ConstructionScript)