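; BP_Money is an interactable money pickup for the inventory system.
; When an actor begins overlapping it, it runs the parent overlap logic, then rolls a random MoneyValue within a small fixed range.
; Interacting adds that value to the passed inventory's Money and destroys the pickup.
; The construction script tints its four cube meshes by pushing the Color variable into their material "Color" parameter.
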(event EventBeginPlay
  (|CallParentFunction) ; This node is disabled and will not be called.\nDrag off pins to build functionality.
)

(event Collision|EventActorBeginOverlap
  (params (OtherActor :type Actor%20Object%20Reference))
  (|CallParentFunction OtherActor)
  (Variables|Default|SetMoneyValue (Math|Random|RandomIntegerinRange 5 10)))

(event EventTick
  (params (DeltaSeconds :type Float%20%28single-precision%29))
  (|CallParentFunction DeltaSeconds) ; This node is disabled and will not be called.\nDrag off pins to build functionality.
)

(event EventInteracting
  (params (PlayerRef :type Third%20Person%20Character%20Object%20Reference) (InventoryRef :type BP%20Invetory%20Object%20Reference))
  (Variables|/Game/GameDesign/JeanDavalos/InvetorySystem/BP_Invetory.BP_Invetory_C|SetMoney InventoryRef (+ (Variables|/Game/GameDesign/JeanDavalos/InvetorySystem/BP_Invetory.BP_Invetory_C|GetMoney InventoryRef) (Variables|Default|GetMoneyValue)))
  (Actor|DestroyActor))

(fn ConstructionScript
  (|CallParentFunction)
  (Rendering|Material|SetVectorParameterValueonMaterials (Variables|Default|GetCube) "Color" (Math|Conversions|ToVector(LinearColor) (Variables|Default|GetColor))))