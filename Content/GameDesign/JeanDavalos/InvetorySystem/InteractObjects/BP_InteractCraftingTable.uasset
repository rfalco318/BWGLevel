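; BP_InteractCraftingTable is an interactable crafting table that turns a sword grip and a sword blade from the inventory into an equipped sword.
; On Interacting it stores the player and inventory references, then checks that both part counts are above zero.
; If so, it spawns BP_EquipSword, snaps it to the player mesh's RightHand socket, prints its name and subtracts one blade and one grip.
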(event EventBeginPlay
  (|CallParentFunction) ; This node is disabled and will not be called.\nDrag off pins to build functionality.
)

(event Collision|EventActorBeginOverlap
  (params (OtherActor :type Actor%20Object%20Reference))
  (|CallParentFunction OtherActor) ; This node is disabled and will not be called.\nDrag off pins to build functionality.
)

(event EventTick
  (params (DeltaSeconds :type Float%20%28single-precision%29))
  (|CallParentFunction DeltaSeconds) ; This node is disabled and will not be called.\nDrag off pins to build functionality.
)

(event EventInteracting
  (params (PlayerRef :type Third%20Person%20Character%20Object%20Reference) (InventoryRef :type BP%20Invetory%20Object%20Reference))
  (Variables|Default|SetPlayer%20Ref PlayerRef)
  (Variables|Default|SetInventory%20Ref InventoryRef)
  (if (and (> (Variables|/Game/GameDesign/JeanDavalos/InvetorySystem/BP_Invetory.BP_Invetory_C|GetSwordGrip (Variables|Default|GetInventory%20Ref)) 0.0) (> (Variables|/Game/GameDesign/JeanDavalos/InvetorySystem/BP_Invetory.BP_Invetory_C|GetSwordBlade (Variables|Default|GetInventory%20Ref)) 0.0))
    (Utilities|FlowControl|Sequence
      (:then_0
        (bind _returnvalue (Game|SpawnActorfromClass "/Game/GameDesign/JeanDavalos/Equip/BP_EquipSword.BP_EquipSword_C" (Transformation|GetWorldTransform (Variables|/Script/Engine.Character|GetMesh (Variables|Default|GetPlayer%20Ref))) "Undefined" 0 0))
        (Transformation|AttachComponentToComponent (Variables|/Script/Engine.Actor|GetRootComponent _returnvalue) (Variables|/Script/Engine.Character|GetMesh (Variables|Default|GetPlayer%20Ref)) "RightHand" "SnapToTarget" "SnapToTarget" "SnapToTarget" true)
        (Development|PrintString (Utilities|GetDisplayName _returnvalue)))
      (:then_1
        (Default|SubtractASwordBlade (Variables|Default|GetInventory%20Ref))
        (Default|SubtractASwordGrip (Variables|Default|GetInventory%20Ref))))))

(fn ConstructionScript
  (|CallParentFunction))