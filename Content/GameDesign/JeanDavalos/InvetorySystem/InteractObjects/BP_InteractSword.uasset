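; BP_InteractSword is an interactable sword object that equips the player with a sword.
; Its Interacting event spawns a BP_EquipSword, snaps it to the RightHand socket on the player's mesh and prints its name.
; Collision sphere overlaps with actors tagged Player show and hide a text render prompt.
; The interactable itself stays in place, with no guard against spawning another sword on repeated interaction.
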(event OnComponentBeginOverlap(CollisionSphere)
  (params (OverlappedComponent :type Primitive%20Component%20Object%20Reference) (OtherActor :type Actor%20Object%20Reference) (OtherComp :type Primitive%20Component%20Object%20Reference) (OtherBodyIndex :type Integer) (bFromSweep :type Boolean) (SweepResult :type Hit%20Result%20Structure%20%28by%20ref%29))
  (if (Actor|ActorHasTag OtherActor "Player")
    (Rendering|SetVisibility (Variables|Default|GetTextRender) true false)))

(event OnComponentEndOverlap(CollisionSphere)
  (params (OverlappedComponent :type Primitive%20Component%20Object%20Reference) (OtherActor :type Actor%20Object%20Reference) (OtherComp :type Primitive%20Component%20Object%20Reference) (OtherBodyIndex :type Integer))
  (if (Actor|ActorHasTag OtherActor "Player")
    (Rendering|SetVisibility (Variables|Default|GetTextRender) false false)))

(event EventInteracting
  (params (PlayerRef :type Third%20Person%20Character%20Object%20Reference) (InventoryRef :type BP%20Invetory%20Object%20Reference))
  (bind _mesh (Variables|/Script/Engine.Character|GetMesh PlayerRef))
  (bind _returnvalue (Game|SpawnActorfromClass "/Game/GameDesign/JeanDavalos/Equip/BP_EquipSword.BP_EquipSword_C" (Transformation|GetWorldTransform _mesh) "Undefined" 0 0))
  (Transformation|AttachComponentToComponent (Variables|/Script/Engine.Actor|GetRootComponent _returnvalue) _mesh "RightHand" "SnapToTarget" "SnapToTarget" "SnapToTarget" true)
  (Development|PrintString (Utilities|GetDisplayName _returnvalue)))

(fn ConstructionScript
  (|CallParentFunction))