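; BP_InteractShield is an interactable shield object in the inventory system that equips a shield on the player when picked up.
; Its PickUpObject event spawns a BP_EquipShield at the player mesh transform and snaps it to the LeftHand socket.
; It prints the new shield's name, and the graph neither destroys the pickup nor records it in an inventory.
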(event EventBeginPlay
  (|CallParentFunction) ; This node is disabled and will not be called.\nDrag off pins to build functionality.
)

(event Collision|EventActorBeginOverlap
  (params (OtherActor :type Actor%20Object%20Reference))
  (|CallParentFunction OtherActor) ; This node is disabled and will not be called.\nDrag off pins to build functionality.
)

(event EventTick
  (params (DeltaSeconds :type Float%20%28single-precision%29))
  (|CallParentFunction DeltaSeconds) ; This node is disabled and will not be called.\nDrag off pins to build functionality.
)

(event EventPickUpObject
  (params (PlayerRef :type Third%20Person%20Character%20Object%20Reference))
  (bind _mesh (Variables|/Script/Engine.Character|GetMesh PlayerRef))
  (bind _returnvalue (Game|SpawnActorfromClass "/Game/GameDesign/JeanDavalos/Equip/BP_EquipShield.BP_EquipShield_C" (Transformation|GetWorldTransform _mesh) "Undefined" 0 0))
  (Transformation|AttachComponentToComponent (Variables|/Script/Engine.Actor|GetRootComponent _returnvalue) _mesh "LeftHand" "SnapToTarget" "SnapToTarget" "SnapToTarget" true)
  (Development|PrintString (Utilities|GetDisplayName _returnvalue)))

(fn ConstructionScript
  (|CallParentFunction))