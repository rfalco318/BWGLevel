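; BP_ContrabandCach1 is an interactable contraband cache that the player can open once.
; Its collision sphere detects Player-tagged actors, registering the cache as the character's interact object and toggling the HUD prompt while it is closed.
; The Interacting event marks it open, plays the S_OpenContrabandCach level sequence paused at its end, then disables interaction and hides the prompt.
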(event OnComponentBeginOverlap(CollisionSphere)
  (params (OverlappedComponent :type Primitive%20Component%20Object%20Reference) (OtherActor :type Actor%20Object%20Reference) (OtherComp :type Primitive%20Component%20Object%20Reference) (OtherBodyIndex :type Integer) (bFromSweep :type Boolean) (SweepResult :type Hit%20Result%20Structure%20%28by%20ref%29))
  (if (and (Actor|ActorHasTag OtherActor "Player") (not (Variables|Default|GetIsOpen?)))
    (Variables|/Game/ThirdPersonBP/Blueprints/ThirdPersonCharacter.ThirdPersonCharacter_C|SetCanInteract? (Variables|Default|GetCharacterRef) true)
    (Variables|/Game/ThirdPersonBP/Blueprints/ThirdPersonCharacter.ThirdPersonCharacter_C|SetBp_InteractObjects (Variables|Default|GetCharacterRef) self)
    (Widget|SetVisibility (Variables|/Game/GameDesign/JeanDavalos/HUDandUI/W_PlayerHud.W_PlayerHud_C|GetOnScreenCanInteract (Variables|/Game/ThirdPersonBP/Blueprints/ThirdPersonCharacter.ThirdPersonCharacter_C|GetCharacterHudRef (Variables|Default|GetCharacterRef))) "Visible")))

(event OnComponentEndOverlap(CollisionSphere)
  (params (OverlappedComponent :type Primitive%20Component%20Object%20Reference) (OtherActor :type Actor%20Object%20Reference) (OtherComp :type Primitive%20Component%20Object%20Reference) (OtherBodyIndex :type Integer))
  (if (and (Actor|ActorHasTag OtherActor "Player") (not (Variables|Default|GetIsOpen?)))
    (Variables|/Game/ThirdPersonBP/Blueprints/ThirdPersonCharacter.ThirdPersonCharacter_C|SetCanInteract? (Variables|Default|GetCharacterRef) false)
    (Variables|/Game/ThirdPersonBP/Blueprints/ThirdPersonCharacter.ThirdPersonCharacter_C|SetBp_InteractObjects (Variables|Default|GetCharacterRef) 0)
    (Widget|SetVisibility (Variables|/Game/GameDesign/JeanDavalos/HUDandUI/W_PlayerHud.W_PlayerHud_C|GetOnScreenCanInteract (Variables|/Game/ThirdPersonBP/Blueprints/ThirdPersonCharacter.ThirdPersonCharacter_C|GetCharacterHudRef (Variables|Default|GetCharacterRef))) "Hidden")))

(event EventBeginPlay
  (|CallParentFunction) ; This node is disabled and will not be called.\nDrag off pins to build functionality.
)

(event Collision|EventActorBeginOverlap
  (params (OtherActor :type Actor%20Object%20Reference))
  (|CallParentFunction OtherActor) ; This node is disabled and will not be called.\nDrag off pins to build functionality.
)

(event EventTick
  (params (DeltaSeconds :type Float%20%28single-precision%29))
  (|CallParentFunction DeltaSeconds) ; This node is disabled and will not be called.\nDrag off pins to build functionality.
)

(event EventInteracting
  (params (PlayerRef :type Third%20Person%20Character%20Object%20Reference) (InventoryRef :type BP%20Invetory%20Object%20Reference))
  (if (not (Variables|Default|GetIsOpen?))
    (Variables|Default|SetIsOpen? true)
    (Sequencer|Player|CreateLevelSequencePlayer "/Game/GameDesign/JeanDavalos/InvetorySystem/InteractObjects/ContrabandCach/S_OpenContrabandCach.S_OpenContrabandCach" (Utilities|Struct|MakeMovieSceneSequencePlaybackSettings true "(Value=0)" 1.0 0.0 false false false false false false false true))
    (Variables|/Game/ThirdPersonBP/Blueprints/ThirdPersonCharacter.ThirdPersonCharacter_C|SetCanInteract? (Variables|Default|GetCharacterRef) false)
    (Widget|SetVisibility (Variables|/Game/GameDesign/JeanDavalos/HUDandUI/W_PlayerHud.W_PlayerHud_C|GetOnScreenCanInteract (Variables|/Game/ThirdPersonBP/Blueprints/ThirdPersonCharacter.ThirdPersonCharacter_C|GetCharacterHudRef (Variables|Default|GetCharacterRef))) "Hidden")))

(fn ConstructionScript
  (|CallParentFunction))