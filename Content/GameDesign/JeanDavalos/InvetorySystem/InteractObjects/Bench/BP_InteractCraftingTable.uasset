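; Interactable crafting table actor that opens the crafting bench UI when the player interacts with it.
; The Interacting event creates a W_CraftingBench widget for player 0, adds it to the viewport and stores the player and inventory references.
; A collision sphere shows the text prompt while an actor tagged Player overlaps it and hides it on exit.
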(event OnComponentBeginOverlap(CollisionSphere)
  (params (OverlappedComponent :type Primitive%20Component%20Object%20Reference) (OtherActor :type Actor%20Object%20Reference) (OtherComp :type Primitive%20Component%20Object%20Reference) (OtherBodyIndex :type Integer) (bFromSweep :type Boolean) (SweepResult :type Hit%20Result%20Structure%20%28by%20ref%29))
  (if (Actor|ActorHasTag OtherActor "Player")
    (Rendering|SetVisibility (Variables|Default|GetTextRender) true false)))

(event OnComponentEndOverlap(CollisionSphere)
  (params (OverlappedComponent :type Primitive%20Component%20Object%20Reference) (OtherActor :type Actor%20Object%20Reference) (OtherComp :type Primitive%20Component%20Object%20Reference) (OtherBodyIndex :type Integer))
  (if (Actor|ActorHasTag OtherActor "Player")
    (Rendering|SetVisibility (Variables|Default|GetTextRender) false false)))

(event EventBeginPlay
  (|CallParentFunction) ; This node is disabled and will not be called.\nDrag off pins to build functionality.
)

(event Collision|EventActorBeginOverlap
  (params (OtherActor :type Actor%20Object%20Reference))
  (|CallParentFunction OtherActor) ; This node is disabled and will not be called.\nDrag off pins to build functionality.
)

(event EventTick
  (params (DeltaSeconds :type Float%20%28single-precision%29))
  (|CallParentFunction DeltaSeconds) ; This node is disabled and will not be called.\nDrag off pins to build functionality.
)

(event EventInteracting
  (params (PlayerRef :type Third%20Person%20Character%20Object%20Reference) (InventoryRef :type BP%20Invetory%20Object%20Reference))
  (bind _returnvalue (UserInterface|CreateWidget "/Game/GameDesign/JeanDavalos/InvetorySystem/InteractObjects/Bench/W_CraftingBench.W_CraftingBench_C" (Game|GetPlayerController 0)))
  (UserInterface|Viewport|AddtoViewport _returnvalue 0)
  (Variables|Default|SetPlayer%20Ref PlayerRef)
  (Variables|Default|SetInventory%20Ref InventoryRef))

(fn ConstructionScript
  (|CallParentFunction))