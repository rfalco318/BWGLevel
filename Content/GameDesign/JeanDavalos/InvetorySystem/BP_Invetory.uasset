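; BP_Invetory is a simple crafting-component inventory that tracks counts of sword grips, sword blades and metal pieces.
; Each component has its own counter variable with a pair of custom events that add or remove one unit.
; Every event prints the new count for debugging, and removal has no lower-bound check, so nothing in the graph prevents negative counts.
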(event EventRemoveOneSwordBlade
  ;[1 1 1] Remove Components from the Inventory
  (bind _result (Math|Integer|DecrementInt (Variables|Default|GetSwordBlade))
    (:%20%20
      (bind _output_get (Variables|Default|SetSwordBlade _result))
      (Development|PrintString (Utilities|String|ToString(Integer) _output_get)))))

(event EventRemoveOneSwordGrip
  ;[1 1 1] Remove Components from the Inventory
  (bind _result (Math|Integer|DecrementInt (Variables|Default|GetSwordGrip))
    (:%20%20
      (bind _output_get (Variables|Default|SetSwordGrip _result))
      (Development|PrintString (Utilities|String|ToString(Integer) _output_get)))))

(event EventAddMetalPiece
  ;[1 1 1] Add Components to the Inventory
  (bind _result (Math|Integer|IncrementInt (Variables|Default|GetMetalPiece))
    (:%20%20
      (bind _output_get (Variables|Default|SetMetalPiece _result))
      (Development|PrintString (Utilities|String|ToString(Integer) _output_get)))))

(event EventAddSwordBlade
  ;[1 1 1] Add Components to the Inventory
  (bind _result (Math|Integer|IncrementInt (Variables|Default|GetSwordBlade))
    (:%20%20
      (bind _output_get (Variables|Default|SetSwordBlade _result))
      (Development|PrintString (Utilities|String|ToString(Integer) _output_get)))))

(event EventAddSwordGrip
  ;[1 1 1] Add Components to the Inventory
  (bind _result (Math|Integer|IncrementInt (Variables|Default|GetSwordGrip))
    (:%20%20
      (bind _output_get (Variables|Default|SetSwordGrip _result))
      (Development|PrintString (Utilities|String|ToString(Integer) _output_get)))))

(event EventRemoveOneMetalPiece
  ;[1 1 1] Remove Components from the Inventory
  (bind _result (Math|Integer|DecrementInt (Variables|Default|GetMetalPiece))
    (:%20%20
      (bind _output_get (Variables|Default|SetMetalPiece _result))
      (Development|PrintString (Utilities|String|ToString(Integer) _output_get)))))

(fn ConstructionScript)