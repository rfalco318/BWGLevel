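; BP_Helmet is a helmet pickup that attaches to the player's character mesh when picked up.
; Its PickUpObject event receives a player reference and attaches the helmet's SkeletalMesh component to that player's Mesh at the "Helmet" socket, snapping location, rotation and scale.
; The Blueprint contains no other active logic, and its construction script only calls the parent.
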(event EventBeginPlay
  (|CallParentFunction) ; This node is disabled and will not be called.\nDrag off pins to build functionality.
)

(event Collision|EventActorBeginOverlap
  (params (OtherActor :type Actor%20Object%20Reference))
  (|CallParentFunction OtherActor) ; This node is disabled and will not be called.\nDrag off pins to build functionality.
)

(event EventTick
  (params (DeltaSeconds :type Float%20%28single-precision%29))
  (|CallParentFunction DeltaSeconds) ; This node is disabled and will not be called.\nDrag off pins to build functionality.
)

(event EventPickUpObject
  (params (PlayerRef :type Third%20Person%20Character%20Object%20Reference))
  (Transformation|AttachComponentToComponent (Variables|Default|GetSkeletalMesh) (Variables|/Script/Engine.Character|GetMesh PlayerRef) "Helmet" "SnapToTarget" "SnapToTarget" "SnapToTarget" true))

(fn ConstructionScript
  (|CallParentFunction))