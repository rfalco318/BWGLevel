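; Enemy pawn Blueprint that roams at random and chases the first-person player character when it sees them.
; Pawn sensing sets CanSeePlayer and starts an AI move toward the player, clearing the flag when the move succeeds or fails.
; Tick runs through a three-second Delay, then moves to a random reachable nearby point unless chasing.
; GetRandomLocation picks a random patrol point index, but the event graph never calls it.
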(event OnSeePawn(PawnSensing)
  (params (Pawn :type Pawn%20Object%20Reference))
  (bind _asfirst_person_character (Utilities|Casting|CastToFirstPersonCharacter Pawn))
  (Variables|Default|SetCanSeePlayer true)
  (AI|AIMoveTo self "0, 0, 0" _asfirst_person_character 5.0 false
    (:OnSuccess
      _)
    (:OnFail
      _))
  (Variables|Default|SetCanSeePlayer false))

(event EventTick
  (params (DeltaSeconds :type Float%20%28single-precision%29))
  (Utilities|FlowControl|Delay 3.0)
  (if (not (Variables|Default|GetCanSeePlayer))
    (AI|AIMoveTo self (.RandomLocation (AI|Navigation|GetRandomReachablePointinRadius (Transformation|GetActorLocation) 1e+03 0 0)) 0 5.0 false)))

(fn ConstructionScript)

(fn GetRandomLocation
  (Variables|Default|SetcurrentPatrolPoint (Math|Random|RandomInteger (Utilities|Array|Length (Variables|Default|GetpatrolPoints)))))